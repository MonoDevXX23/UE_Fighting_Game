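; BP_Player is a flipbook-animated player character with running, punch and sword inputs.
; On BeginPlay it adds the default Enhanced Input mapping context through BP_PlayerControl.
; Run input moves it along the actor's forward vector, switches to the run flipbook and rotates the sprite to face the input's sign.
; Attacks only play their flipbook, returning to idle after a fixed delay, with no hit logic.
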(event `self.ReceiveBeginPlay`
  (bind _asbp_player_control (cast `/Game/Blueprints/BP_PlayerControl` (`self.GetController`)))
  (`EnhancedInputSubsystemInterface.AddMappingContext` (pcsubsystem `EnhancedInputLocalPlayerSubsystem` _asbp_player_control) "/Game/Blueprints/IMC_Default.IMC_Default" 0 (struct)))

(event `EnhancedInput|/Game/Blueprints/InputActions/IA_Run`
  (params (ActionValue :type "Float (double-precision)") (ElapsedSeconds :type "Float (double-precision)") (TriggeredSeconds :type "Float (double-precision)") (InputAction :type "InputAction Object Reference" :default "/Game/Blueprints/InputActions/IA_Run.IA_Run"))
  ;[1 1 1] Anmation - Run
  (:`Triggered`
    (`self.AddMovementInput` (`self.GetActorForwardVector`) ActionValue)
    (`PaperFlipbookComponent.SetFlipbook` (`self.Sprite`) "/Game/Assets/Textures/Characters/Player/Run/FB_Run.FB_Run")
    (if (> ActionValue 0.0)
      (`SceneComponent.K2_SetWorldRotation` :`self` (`self.Sprite`))
      (else
        (`SceneComponent.K2_SetWorldRotation` (`self.Sprite`) (struct :`Yaw` -180.0) false false))))
  (:`Completed`
    (`PaperFlipbookComponent.SetFlipbook` (`self.Sprite`) "/Game/Assets/Textures/Characters/Player/Idle/FB_Idle.FB_Idle")))

(event `EnhancedInput|/Game/Blueprints/InputActions/IA_Attack`
  (params (ActionValue :type Boolean) (ElapsedSeconds :type "Float (double-precision)") (TriggeredSeconds :type "Float (double-precision)") (InputAction :type "InputAction Object Reference" :default "/Game/Blueprints/InputActions/IA_Attack.IA_Attack"))
  ;[1 1 1] Attack - 1 (Punch)
  (:`Triggered`
    (`PaperFlipbookComponent.SetFlipbook` (`self.Sprite`) "/Game/Assets/Textures/Characters/Player/Attack/Cross_Punch/FB_Punch.FB_Punch")
    (`KismetSystemLibrary.Delay` 0.8)
    (`PaperFlipbookComponent.SetFlipbook` (`self.Sprite`) "/Game/Assets/Textures/Characters/Player/Idle/FB_Idle.FB_Idle")))

(event `EnhancedInput|/Game/Blueprints/InputActions/IA_Sword1`
  (params (ActionValue :type Boolean) (ElapsedSeconds :type "Float (double-precision)") (TriggeredSeconds :type "Float (double-precision)") (InputAction :type "InputAction Object Reference" :default "/Game/Blueprints/InputActions/IA_Sword1.IA_Sword1"))
  ;[1 1 1] Attack - 2 (Sword)
  (:`Triggered`
    (`PaperFlipbookComponent.SetFlipbook` (`self.Sprite`) "/Game/Assets/Textures/Characters/Player/Attack/Sword_Attack/FB_Sword1.FB_Sword1")
    (`KismetSystemLibrary.Delay` 0.45)
    (`PaperFlipbookComponent.SetFlipbook` (`self.Sprite`) "/Game/Assets/Textures/Characters/Player/Idle/FB_Idle.FB_Idle")))

(fn `UserConstructionScript`)