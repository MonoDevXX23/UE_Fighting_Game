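; AI spawner actor that repeatedly spawns enemy AI at its Billboard component's location.
; On BeginPlay, if the enemy count is below the maximum, it enters a delayed loop that spawns and increments the count without rechecking the limit.
; EnemyCounter binds CountEnemies to a passed-in enemy's event, which decrements the count when triggered.
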(event `self.ReceiveBeginPlay`
  (if (< (`self.Current_Enemy_Count`) (`self.Max_Enemies`))
    (`KismetSystemLibrary.Delay` (`self.Duration`))
    (`AIBlueprintHelperLibrary.SpawnAIFromClass` "/Game/Blueprints/PaperZD/Enemy/Enemy.Enemy_C" null (`SceneComponent.K2_GetComponentLocation` (`self.Billboard`)) (struct) false null :!label _label)
    (`KismetSystemLibrary.Delay` (`self.Duration`))
    (set `self.Current_Enemy_Count` (+ (`self.Current_Enemy_Count`) 1.0))
    (goto _label)))

(event `EnemyCounter`
  (params (Enemy_Ref :type "/Game/Blueprints/PaperZD/Enemy/Enemy Object Reference"))
  (bind _output_get (set `self.Enemy_ref` Enemy_Ref))
  (if (`KismetSystemLibrary.IsValid` _output_get)
    (add `/Game/Blueprints/PaperZD/Enemy/Enemy.EnemyCount` (`self.Enemy_ref`) (delegate `CountEnemies`))
    (`KismetSystemLibrary.PrintString` "Bound Enemy COunt" true true (struct :`R` 0.516667 :`G` 0.003543 :`A` 1.0))))

(event `CountEnemies`
  (set `self.Current_Enemy_Count` (- (`self.Current_Enemy_Count`) 1.0)))

(fn `UserConstructionScript`)